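; Energy beam emitter actor that fires a selectable laser, electro laser, electric arc or pulse beam, bouncing it off reflective surfaces.
; BeginPlay pools one particle beam per allowed bounce, tinted and sized from its settings.
; While active, each Tick runs a recursive line trace, reflecting only off GameTraceChannel1 objects.
; Segments position the pooled beams, hiding extras, spawn optional sparks and burn decals, and report the last hit actor through OnLaserHit.
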(event EventBeginPlay
  ;[1 1 1] Spawn all the emiters as defined in the maximum energy beam / ray reflection variable, based on the selected type
  (Utilities|Array|Clear (Variables|Default|GetBeamArray))
  (for _index (range 1 (Math|Conversions|ToInteger(Byte) (Variables|EnergyBeam/RayEmiter|GetMax%20Bounces)))
    (switch Utilities|FlowControl|Switch|SwitchonE_EnergyBeamTypes (Variables|EnergyBeam/RayEmiter|GetEnergy%20Beam%20/%20Ray%20Type)
      (:NewEnumerator0
        (Variables|Default|SetEnergyType "/Game/Utilities/ULASER/Particles/P_Laser.P_Laser"))
      (:NewEnumerator1
        (Variables|Default|SetEnergyType "/Game/Utilities/ULASER/Particles/P_ElectroLaser.P_ElectroLaser"))
      (:NewEnumerator2
        (Variables|Default|SetEnergyType "/Game/Utilities/ULASER/Particles/P_ElectricArc.P_ElectricArc"))
      (:NewEnumerator3
        (Variables|Default|SetEnergyType "/Game/Utilities/ULASER/Particles/P_PulseBeam.P_PulseBeam")))
    (bind _returnvalue (Effects|SpawnEmitterAttached (Variables|Default|GetEnergyType) (Variables|Default|GetScene) "None" "0, 0, 0" "0, 0, 0" "1.000000,1.000000,1.000000" "KeepWorldPosition" false))
    (Utilities|Array|Add (Variables|Default|GetBeamArray) _returnvalue)
    (Effects|Components|ParticleSystem|SetVectorParameter _returnvalue "InstanceColorScaleOverLife" (Math|Conversions|ToVector(LinearColor) (Variables|EnergyBeam/RayEmiter|GetEnergy%20Beam%20Color)))
    (Effects|Components|ParticleSystem|SetVectorParameter _returnvalue "InstanceInitalSize" (Math|Conversions|ToVector(Float) (Variables|EnergyBeam/RayEmiter|GetEnergy%20Beam%20Girth)))))

(event EventTick
  (params (DeltaSeconds :type Float%20%28single-precision%29))
  (bind _scene (Variables|Default|GetScene))
  (bind _energy_beam_girth (Variables|EnergyBeam/RayEmiter|GetEnergy%20Beam%20Girth))
  (bind _returnvalue (/ _energy_beam_girth 1e+01))
  (bind _returnvalue_2 (Math|Conversions|ToVector(Float) _returnvalue))
  ;[1 1 1] Check for collision every tick and draw the "max bounces" number of particle beams accordingly
  (Variables|Default|SetCounter (Variables|EnergyBeam/RayEmiter|GetMax%20Bounces))
  (Utilities|Array|Clear (Variables|Default|GetBeamVectorArray))
  (Variables|Default|SetLastHitActor 0)
  (if (Variables|EnergyBeam/RayEmiter|GetActive)
    (CallFunction|CheckCollision (Transformation|GetWorldLocation _scene) (Math|Vector|GetForwardVector (Transformation|GetWorldRotation _scene)))
    (for (_array_element _array_index) (Variables|Default|GetBeamArray)
      (Variables|Default|SetBeam _array_element)
      (if (< _array_index (Utilities|Array|Length (Variables|Default|GetBeamVectorArray)))
        (Rendering|SetVisibility (Variables|Default|GetBeam) true false)
        (Transformation|SetWorldLocation (Variables|Default|GetBeam) (.v1 (Utilities|Struct|BreakTwoVectors (Utilities|Array|Get(acopy) (Variables|Default|GetBeamVectorArray) _array_index))) false false)
        (if (Variables|SpecialFX|GetGenerate%20Sparks%20on%20Impact)
          (bind _returnvalue_3 (Effects|SpawnEmitteratLocation "/Game/Utilities/ULASER/Particles/P_Sparks.P_Sparks" (.v2 (Utilities|Struct|BreakTwoVectors (Utilities|Array|Get(acopy) (Variables|Default|GetBeamVectorArray) _array_index))) (Class|KismetMathLibrary|NegateRotator (Math|Conversions|RotationFromXVector (.v2 (Utilities|Struct|BreakTwoVectors (Utilities|Array|Get(acopy) (Variables|Default|GetBeamVectorArray) _array_index))))) _returnvalue_2))
          (Effects|Components|ParticleSystem|SetVectorParameter _returnvalue_3 "SparksColor" (* (Math|Conversions|ToVector(LinearColor) (Variables|EnergyBeam/RayEmiter|GetEnergy%20Beam%20Color)) 1e+02))
          (if (Variables|SpecialFX|GetGenerate%20Burn%20Marks%20/%20Trail)
            (Rendering|Decal|SpawnDecalatLocation "/Game/Utilities/ULASER/Materials/M_BurnMark.M_BurnMark" (* _returnvalue_2 5e+01) (.v2 (Utilities|Struct|BreakTwoVectors (Utilities|Array|Get(acopy) (Variables|Default|GetBeamVectorArray) _array_index))) (Class|KismetMathLibrary|NegateRotator (Math|Conversions|RotationFromXVector (.v2 (Utilities|Struct|BreakTwoVectors (Utilities|Array|Get(acopy) (Variables|Default|GetBeamVectorArray) _array_index))))) 1.0)
            (if true
              (Effects|SpawnEmitteratLocation 0 (.v2 (Utilities|Struct|BreakTwoVectors (Utilities|Array|Get(acopy) (Variables|Default|GetBeamVectorArray) _array_index))) (Class|KismetMathLibrary|NegateRotator (Math|Conversions|RotationFromXVector (.v2 (Utilities|Struct|BreakTwoVectors (Utilities|Array|Get(acopy) (Variables|Default|GetBeamVectorArray) _array_index))))) _returnvalue_2))))
        (Class|ParticleSystemComponent|SetBeamEndPoint (Variables|Default|GetBeam) 0 (.v2 (Utilities|Struct|BreakTwoVectors (Utilities|Array|Get(acopy) (Variables|Default|GetBeamVectorArray) _array_index))))
        (Default|CallOnLaserHit (Variables|Default|GetLastHitActor))
        (else
          (Rendering|SetVisibility (Variables|Default|GetBeam) false false))))))

(fn ConstructionScript
  (bind _cube (Variables|Default|GetCube))
  (if (!= (Variables|EnergyBeam/RayEmiter|GetEnergy%20Beam%20Emiter%20Mesh) 0)
    (Components|StaticMesh|SetStaticMesh _cube (Variables|EnergyBeam/RayEmiter|GetEnergy%20Beam%20Emiter%20Mesh))
    (Rendering|Material|SetMaterial _cube 0 0)))

(fn CheckCollision
  (params (Location :type Vector) (Forward :type Vector))
  (bind _output_get (LocalVariables|SetLaserVector (Utilities|Struct|MakeTwoVectors (+ Location (* Forward 1.0)) (+ Location (* Forward (Variables|EnergyBeam/RayEmiter|GetMax%20Render%20Distance))))))
  (bind _outhit (Collision|LineTraceByChannel (.v1 _output_get) (.v2 _output_get) "TraceTypeQuery1" false 0 "None"))
  (if (.bBlockingHit (Collision|BreakHitResult _outhit))
    (Variables|Default|SetLastHitActor (.HitActor (Collision|BreakHitResult _outhit)))
    (LocalVariables|SetLaserVector (Utilities|Struct|MakeTwoVectors (.TraceStart (Collision|BreakHitResult _outhit)) (.ImpactPoint (Collision|BreakHitResult _outhit))))
    (if (Utilities|Enum|Equal(Enum) (Collision|GetCollisionObjectType (.HitComponent (Collision|BreakHitResult _outhit))) "ECC_GameTraceChannel1")
      (Utilities|Array|Add (Variables|Default|GetBeamVectorArray) (LocalVariables|GetLaserVector))
      (bind _output_get_2 (Variables|Default|SetCounter (Math|Conversions|ToByte(Integer) (- (Math|Conversions|ToInteger(Byte) (Variables|Default|GetCounter)) 1))))
      (if (> (Math|Conversions|ToInteger(Byte) _output_get_2) 0)
        (CallFunction|CheckCollision (.ImpactPoint (Collision|BreakHitResult _outhit)) (Math|Vector|GetReflectionVector (Math|Vector|GetUnitDirection(Vector) (.TraceStart (Collision|BreakHitResult _outhit)) (.TraceEnd (Collision|BreakHitResult _outhit))) (.Normal (Collision|BreakHitResult _outhit))))
        (else
          (return)))
      (else
        (Utilities|Array|Add (Variables|Default|GetBeamVectorArray) (LocalVariables|GetLaserVector) :!label _label)
        (return)))
    (else
      (goto _label))))