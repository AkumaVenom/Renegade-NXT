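; Parent character Blueprint for GDI soldiers, delegating combat to a RenegadeSoldierCombat component and adding movement and lock-on control.
; Combat start and end events toggle spline combat state for the actor, with combat start also setting run speed.
; Sprint input raises walk speed unless stationary, reloading or firing, and Tick cancels it once when a player-controlled soldier stops.
; Lock-on input toggles targeting, which respawn clears along with resetting walk speed.
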(event OnCombatStarted(RenegadeSoldierCombat)
  (params (Target :type Actor%20Object%20Reference))
  (Variables|/Script/Engine.CharacterMovementComponent|SetMaxWalkSpeed (Variables|Character|GetCharacterMovement) 6e+02)
  (Class|RenegadeSplineAIBlueprintLibrary|SetSplineCombatActiveforActor self true Target -1.0))

(event OnCombatEnded(RenegadeSoldierCombat)
  (params (PreviousTarget :type Actor%20Object%20Reference) (ResumeFromLocation :type Vector :default "0, 0, 0"))
  (Class|RenegadeSplineAIBlueprintLibrary|SetSplineCombatActiveforActor self false 0 -1.0))

(event OnRespawned(RenegadeSoldierCombat)
  (Variables|/Script/Engine.CharacterMovementComponent|SetMaxWalkSpeed (Variables|Character|GetCharacterMovement) 6e+02)
  (Class|RenegadeSoldierCombatComponent|PlayerStopLockon (Variables|Default|GetRenegadeSoldierCombat))
  (Variables|Default|SetToggleLockOn false))

(event Custom|StopSprinting
  (Variables|Default|SetIsSprinting false)
  (Variables|/Script/Engine.CharacterMovementComponent|SetMaxWalkSpeed (Variables|Character|GetCharacterMovement) 6e+02))

(event EventBeginPlay)

(event Collision|EventActorBeginOverlap
  (params (OtherActor :type Actor%20Object%20Reference)))

(event EventTick
  (params (DeltaSeconds :type Float%20%28single-precision%29))
  (if (Class|RenegadeSoldierCombatComponent|IsPlayerControlledCombatant (Variables|Default|GetRenegadeSoldierCombat))
    (if (< (Math|Vector|VectorLength (Variables|/Script/Engine.MovementComponent|GetVelocity (Variables|Character|GetCharacterMovement))) 1.0)
      (Utilities|FlowControl|DoOnce false :!label _label
        (:Completed
          (CallFunction|StopSprinting)))
      (else
        (goto _label Reset)))))

(event Input|ActionEvents|InputActionLockOn
  (params (Key :type Key%20Structure :default "None"))
  (bind _renegadesoldiercombat (Variables|Default|GetRenegadeSoldierCombat))
  (:Pressed
    (if (Variables|Default|GetToggleLockOn)
      (Class|RenegadeSoldierCombatComponent|PlayerStopLockon _renegadesoldiercombat)
      (Variables|Default|SetToggleLockOn false)
      (else
        (Variables|Default|SetToggleLockOn true)
        (Class|RenegadeSoldierCombatComponent|PlayerStartLockon _renegadesoldiercombat)))))

(event Input|ActionEvents|InputActionSprint
  (params (Key :type Key%20Structure :default "None"))
  (bind _charactermovement (Variables|Character|GetCharacterMovement))
  (bind _renegadesoldiercombat (Variables|Default|GetRenegadeSoldierCombat))
  (:Pressed
    (if (not (< (Math|Vector|VectorLength (Variables|/Script/Engine.MovementComponent|GetVelocity (Variables|Character|GetCharacterMovement))) 1.0))
      (if (not (or (Class|RenegadeSoldierCombatComponent|IsReloading _renegadesoldiercombat) (Class|RenegadeSoldierCombatComponent|IsPlayerFireHeld _renegadesoldiercombat)))
        (Variables|Default|SetIsSprinting true)
        (Variables|/Script/Engine.CharacterMovementComponent|SetMaxWalkSpeed _charactermovement 1e+03))))
  (:Released
    (Variables|Default|SetIsSprinting false)
    (Variables|/Script/Engine.CharacterMovementComponent|SetMaxWalkSpeed _charactermovement 6e+02)))

(fn ConstructionScript
  (|CallParentFunction))