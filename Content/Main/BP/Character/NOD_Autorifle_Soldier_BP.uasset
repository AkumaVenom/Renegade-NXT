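; Nod autorifle soldier character that follows spline paths and reacts to events from its RenegadeSoldierCombat component.
; Each shot plays a muzzle flash and rifle sound aimed at the trace end, plus blood only when the hit actor is a GDI autorifle soldier.
; When combat ends it resumes path following; on respawn it finds the nearest compatible path and rejoins it from its current location.
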(event OnShotFired(RenegadeSoldierCombat)
  (params (TraceStart :type Vector :default "0, 0, 0") (TraceEnd :type Vector :default "0, 0, 0") (bBlockingHit :type Boolean) (HitResult :type Hit%20Result%20Structure%20%28by%20ref%29))
  (bind _muzzle (Variables|Default|GetMuzzle)
    (:then
      (Effects|SpawnEmitterAttached "/Game/Utilities/ShooterVFXVariety/Particles/P_Shotgun_MuzzleFlash.P_Shotgun_MuzzleFlash" (Variables|Default|GetMuzzle) "None" (Transformation|GetWorldLocation _muzzle) (Math|Rotator|FindLookatRotation (Transformation|GetWorldLocation _muzzle) TraceEnd) "1.000000,1.000000,1.000000" "KeepWorldPosition")
      (Audio|PlaySoundatLocation "/Game/Main/Sound/Weapon/Autorifle/RifleFire_Cue.RifleFire_Cue" (Transformation|GetActorLocation) (Math|Rotator|FindLookatRotation (Transformation|GetWorldLocation _muzzle) TraceEnd) 1.0 1.0 0.0 0 0 self 0)
      (Utilities|Casting|CastToGDI_Autorifle_Soldier_BP (.HitActor (Collision|BreakHitResult HitResult)))
      (Effects|SpawnEmitteratLocation "/Game/Utilities/ShooterVFXVariety/BloodVFX/Particles/Cascade/Real/P_Blood_BulletHit.P_Blood_BulletHit" TraceEnd (Math|Rotator|FindLookatRotation (Transformation|GetWorldLocation _muzzle) TraceEnd) "2.000000,2.000000,2.000000"))
    (:else)))

(event OnCombatEnded(RenegadeSoldierCombat)
  (params (PreviousTarget :type Actor%20Object%20Reference) (ResumeFromLocation :type Vector :default "0, 0, 0"))
  (Class|RenegadeSplineFollowerComponent|ResumeFollowing (Variables|Default|GetRenegadeSplineFollower) true))

(event OnRespawned(RenegadeSoldierCombat)
  (bind _returnvalue (Class|RenegadeSplineAIBlueprintLibrary|FindNearestCompatiblePath (Transformation|GetActorLocation self) 0 "None" 0.0))
  (Class|RenegadeSplineFollowerComponent|StartFollowing (Variables|Default|GetRenegadeSplineFollower) _returnvalue true))

(event EventBeginPlay
  (|CallParentFunction) ; This node is disabled and will not be called.\nDrag off pins to build functionality.
)

(event Collision|EventActorBeginOverlap
  (params (OtherActor :type Actor%20Object%20Reference))
  (|CallParentFunction OtherActor) ; This node is disabled and will not be called.\nDrag off pins to build functionality.
)

(event EventTick
  (params (DeltaSeconds :type Float%20%28single-precision%29))
  (|CallParentFunction DeltaSeconds) ; This node is disabled and will not be called.\nDrag off pins to build functionality.
)

(fn ConstructionScript
  (|CallParentFunction))